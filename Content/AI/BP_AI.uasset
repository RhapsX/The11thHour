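; Enemy AI pawn that roams random reachable points, chases pawns it sees and drains first-person character health on contact.
; Sightings start a looping radio-noise sound once and chase the target; after a retriggerable delay it searches nearby points.
; Finished searches or failed random moves trigger a reset that walks to a fixed point, stops the sound and resumes roaming.
; CatchCollision overlap runs a delayed damage loop until overlap ends.
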(event OnSeePawn(PawnSensing)
  (params (Pawn :type Pawn%20Object%20Reference))
  (Variables|Default|SetisAlert true)
  (if (Variables|Default|GetisSounding)
    _
    (else
      (bind _returnvalue (Audio|SpawnSoundatLocation "/Game/AI/485420__inspectorj__radio-noise-long-wave-01-01-loop.485420__inspectorj__radio-noise-long-wave-01-01-loop" (Transformation|GetActorLocation self) "0, 0, 0" 1.0 1.0 0.0 "/Game/AI/RadioAtten.RadioAtten" 0 false))
      (Variables|Default|SetAlertSound _returnvalue)
      (Variables|Default|SetisSounding true)))
  (Variables|Default|SetInspectCount 0)
  (Utilities|FlowControl|Sequence
    (:then_0
      (AI|AIMoveTo self "0, 0, 0" Pawn 5.0 false))
    (:then_1
      (Utilities|FlowControl|RetriggerableDelay 5.0)
      (CallFunction|RandomInspect))))

(event OnComponentBeginOverlap(CatchCollision)
  (params (OverlappedComponent :type Primitive%20Component%20Object%20Reference) (OtherActor :type Actor%20Object%20Reference) (OtherComp :type Primitive%20Component%20Object%20Reference) (OtherBodyIndex :type Integer) (bFromSweep :type Boolean) (SweepResult :type Hit%20Result%20Structure%20%28by%20ref%29))
  (Variables|Default|SetisCatching true)
  (bind _asbp_first_person_character (Utilities|Casting|CastToBP_FirstPersonCharacter OtherActor))
  (bind _output_get (Variables|/Game/FirstPerson/Blueprints/BP_FirstPersonCharacter.BP_FirstPersonCharacter_C|SetCurrentHealth _asbp_first_person_character (- (Variables|/Game/FirstPerson/Blueprints/BP_FirstPersonCharacter.BP_FirstPersonCharacter_C|GetCurrentHealth _asbp_first_person_character) 2e+01) :!label _label))
  (Default|CallUpdateHealth _asbp_first_person_character _output_get)
  (if (Variables|Default|GetisCatching)
    (Utilities|FlowControl|RetriggerableDelay 1.0)
    (goto _label)))

(event OnComponentEndOverlap(CatchCollision)
  (params (OverlappedComponent :type Primitive%20Component%20Object%20Reference) (OtherActor :type Actor%20Object%20Reference) (OtherComp :type Primitive%20Component%20Object%20Reference) (OtherBodyIndex :type Integer))
  (Variables|Default|SetisCatching false))

(event Custom|Random%20Roam
  (AI|AIMoveTo self (.RandomLocation (AI|Navigation|GetRandomReachablePointinRadius (Transformation|GetActorLocation) 7.5e+02 0 0)) 0 5.0 false
    (:OnSuccess
      (CallFunction|RandomRoam))
    (:OnFail
      (CallFunction|AIReset))))

(event Custom|Random%20Inspect
  (AI|AIMoveTo self (.RandomLocation (AI|Navigation|GetRandomReachablePointinRadius (Transformation|GetActorLocation) 1e+02 0 0)) 0 5.0 false
    (:OnSuccess
      (bind _output_get (Variables|Default|SetInspectCount (+ (Variables|Default|GetInspectCount) 1)))
      (if (> _output_get 3)
        (CallFunction|AIReset)
        (else
          (CallFunction|RandomInspect))))
    (:OnFail
      (CallFunction|AIReset))))

(event Custom|AI%20Reset
  (Variables|Default|SetisAlert false)
  (Variables|Default|SetInspectCount 0)
  (AI|AIMoveTo self "0.000000,0.000000,-84.000000" 0 5.0 false
    (:OnSuccess
      (Audio|Components|Audio|Stop (Variables|Default|GetAlertSound))
      (CallFunction|RandomRoam))))

(event EventBeginPlay
  (CallFunction|RandomRoam))

(fn ConstructionScript)